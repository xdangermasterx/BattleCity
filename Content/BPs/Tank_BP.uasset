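; Tank Blueprint that fires missiles on a cooldown and is destroyed when a missile hits it.
; Fire makes an AI-audible noise, then, if allowed, spawns a Missile_BP at the Arrow component's transform with itself as instigator.
; A one-shot timer set to FireRate calls UpdateFire to re-enable firing.
; A hit on the static mesh by a Missile_BP destroys the tank.
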(event `Fire`
  (`self.MakeNoise` 1.0 self (`self.K2_GetActorLocation`) 0.0 "Fire")
  (if (`self.CanFire`)
    (`|SpawnActorFromClass` "/Game/BPs/Missile_BP.Missile_BP_C" (`SceneComponent.K2_GetComponentToWorld` (`self.Arrow`)) "AdjustIfPossibleButAlwaysSpawn" "OverrideRootScale" null self)
    (set `self.CanFire` false)
    (bind _returnvalue (`KismetSystemLibrary.K2_SetTimerDelegate` (delegate `UpdateFire`) (`self.FireRate`)))
    (set `self.Timer` _returnvalue)))

(event `UpdateFire`
  (set `self.CanFire` true)
  (`KismetSystemLibrary.K2_ClearAndInvalidateTimerHandle` (`self.Timer`)))

(event `self.StaticMesh.OnComponentHit`
  (params (HitComponent :type "PrimitiveComponent Object Reference") (OtherActor :type "Actor Object Reference") (OtherComp :type "PrimitiveComponent Object Reference") (NormalImpulse :type "Vector Structure") (Hit :type "HitResult Structure (by ref)"))
  (cast `/Game/BPs/Missile_BP` OtherActor)
  (`self.K2_DestroyActor`))

(fn `UserConstructionScript`)