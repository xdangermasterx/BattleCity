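; Player Blueprint that moves forward and back, turns, and fires missiles.
; Look input adds controller yaw when the SpringArm uses pawn control rotation; otherwise Turn yaws the actor directly by input times TurnRate.
; Fire input calls Fire, whose body is not in this file, then spawns a Missile_BP at the Arrow component's transform with uniform Scale, owned and instigated by the player.
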(event `Turn`
  (params (Value :type "Float (double-precision)"))
  (`self.K2_SetActorRotation` (`KismetMathLibrary.MakeRotator` 0.0 0.0 (+ (* Value (`self.TurnRate`)) (.yaw (`self.K2_GetActorRotation`))))))

(event `InputAxis|MoveForward`
  (params (AxisValue :type "Float (single-precision)"))
  (`self.AddMovementInput` (`self.GetActorForwardVector`) AxisValue))

(event `InputAxis|LookRight`
  (params (AxisValue :type "Float (single-precision)"))
  (if (`SpringArmComponent.bUsePawnControlRotation` (`self.SpringArm`))
    (`self.AddControllerYawInput` AxisValue)
    (else
      (`self.Turn` AxisValue))))

(event `InputAction|Fire`
  (params (Key :type "Key Structure"))
  (bind _arrow (`self.Arrow`))
  (bind _scale (`self.Scale`))
  (:`Pressed`
    (`self.Fire`)
    (`|SpawnActorFromClass` "/Game/BPs/Missile_BP.Missile_BP_C" (`KismetMathLibrary.MakeTransform` (`SceneComponent.K2_GetComponentLocation` _arrow) (`SceneComponent.K2_GetComponentRotation` _arrow) (`KismetMathLibrary.MakeVector` _scale _scale _scale)) "AdjustIfPossibleButAlwaysSpawn" "OverrideRootScale" self self)))

(fn `UserConstructionScript`)